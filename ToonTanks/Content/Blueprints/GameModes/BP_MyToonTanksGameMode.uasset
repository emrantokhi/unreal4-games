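; BP_MyToonTanksGameMode is the game mode Blueprint for Toon Tanks that handles the game's start, HUD and end screens.
; BeginPlay creates the HUD widget, and both it and the DisplayHUD event feed health, max health and remaining tower count into that widget.
; StartGame shows the start widget, while GameOver shows the end widget with win or loss text chosen by WonGame.
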(event EventBeginPlay
  (bind _returnvalue (UserInterface|CreateWidget "/Game/Blueprints/Widgets/WBP_HUDWidget.WBP_HUDWidget_C"))
  (UserInterface|Viewport|AddtoViewport _returnvalue 0)
  (Variables|/Game/Blueprints/Widgets/WBP_HUDWidget.WBP_HUDWidget_C|SetHealthValue _returnvalue (stale EventDisplayHUD Health))
  (Variables|/Game/Blueprints/Widgets/WBP_HUDWidget.WBP_HUDWidget_C|SetMaxHealthValue _returnvalue (stale EventDisplayHUD MaxHealth))
  (Rendering|Components|TextRender|SetText (Variables|/Game/Blueprints/Widgets/WBP_HUDWidget.WBP_HUDWidget_C|GetNumTowersLeft _returnvalue) (Utilities|Text|ToText(Integer) (stale EventDisplayHUD NumTowers))))

(event EventTick
  (params (DeltaSeconds :type Float%20%28single-precision%29)))

(event EventStartGame
  (bind _returnvalue (UserInterface|CreateWidget "/Game/Blueprints/Widgets/WBP_StartGameWidget.WBP_StartGameWidget_C"))
  (UserInterface|Viewport|AddtoViewport _returnvalue 0))

(event EventGameOver
  (params (bWonGame :type Boolean))
  (bind _returnvalue (UserInterface|CreateWidget "/Game/Blueprints/Widgets/WBP_EndGameWidget.WBP_EndGameWidget_C"))
  (UserInterface|Viewport|AddtoViewport _returnvalue 0)
  (Rendering|Components|TextRender|SetText (Variables|/Game/Blueprints/Widgets/WBP_EndGameWidget.WBP_EndGameWidget_C|GetDisplayText _returnvalue) (select bWonGame "YOU WON!" "YOU LOST!")))

(event EventDisplayHUD
  (params (Health :type Float%20%28single-precision%29) (MaxHealth :type Float%20%28single-precision%29) (NumTowers :type Integer))
  (Variables|/Game/Blueprints/Widgets/WBP_HUDWidget.WBP_HUDWidget_C|SetHealthValue (stale EventBeginPlay _returnvalue) Health)
  (Variables|/Game/Blueprints/Widgets/WBP_HUDWidget.WBP_HUDWidget_C|SetMaxHealthValue (stale EventBeginPlay _returnvalue) MaxHealth)
  (Rendering|Components|TextRender|SetText (Variables|/Game/Blueprints/Widgets/WBP_HUDWidget.WBP_HUDWidget_C|GetNumTowersLeft (stale EventBeginPlay _returnvalue)) (Utilities|Text|ToText(Integer) NumTowers)))

(fn ConstructionScript)